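; WaveBP is a short-lived wave effect actor built on a static mesh that animates once when spawned, then destroys itself.
; The construction script creates a dynamic instance of WaveMat on the mesh.
; On BeginPlay, the Scaling timeline drives both the mesh's uniform scale and, inversely, the material's Translucent parameter, then destroys the actor when finished.
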(event EventBeginPlay
  (bind _value (Timeline|Scaling Play)
    (:Update
      (Transformation|SetRelativeScale3D (Variables|Default|GetStaticMesh) (Math|Conversions|ToVector(Float) _value))
      (Rendering|Material|SetScalarParameterValue (Variables|Default|GetDynamicMat) "Translucent" (- 1.0 _value) :!class /Script/Engine.MaterialInstanceDynamic))
    (:Finished
      (Actor|DestroyActor))))

(event Collision|EventActorBeginOverlap
  (params (OtherActor :type Actor%20Object%20Reference)))

(event EventTick
  (params (DeltaSeconds :type Float%20%28single-precision%29)))

(fn ConstructionScript
  (bind _returnvalue (Rendering|Material|CreateDynamicMaterialInstance (Variables|Default|GetStaticMesh) 0 "/Game/Assets/Material/WaveMat.WaveMat" "WaveMatInst" :!class /Script/Engine.PrimitiveComponent))
  (Variables|Default|SetDynamicMat _returnvalue))