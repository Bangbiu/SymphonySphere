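; SongBP is an actor that builds a song at BeginPlay by spawning a TutorialSphere for each row of its SongData table.
; Row X/Y offset the actor's location, while row Z encodes timing, converted via TimeToHeight at reduced gravity into spawn height.
; A downward trace finds the surface beneath, and height plus a size-based offset is added.
; Spheres attach to the actor and are tracked for DestroyAll, which also destroys the actor.
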(event EventBeginPlay
  (CallFunction|SpawnSong (Variables|Default|GetSongData)))

(event Collision|EventActorBeginOverlap
  (params (OtherActor :type Actor%20Object%20Reference)))

(event EventTick
  (params (DeltaSeconds :type Float%20%28single-precision%29)))

(fn ConstructionScript)

(fn SpawnSong
  (params (InputSong :type Data%20Table%20Object%20Reference))
  (bind _returnvalue (Transformation|GetActorLocation))
  (bind _outrownames (DataTable|GetDataTableRowNames InputSong))
  (for _array_element _outrownames
    (bind _returnvalue_2 (Utilities|GetDataTableRow InputSong _array_element)
      (:then
        (CallFunction|SpawnSphere (Math|Vector|MakeVector (+ (.x (.Position (Utilities|Struct|BreakSphereStruct _returnvalue_2))) (.x _returnvalue)) (+ (.y (.Position (Utilities|Struct|BreakSphereStruct _returnvalue_2))) (.y _returnvalue)) 2e+02) (/ (.z (.Position (Utilities|Struct|BreakSphereStruct _returnvalue_2))) 0.5) (.SphereInfo (Utilities|Struct|BreakSphereStruct _returnvalue_2)))))))

(fn SpawnSphere
  (params (Pos :type Vector) (beat :type Float%20%28double-precision%29) (SI :type Sphere%20Info%20Struct%20Structure))
  (bind _outhit (Collision|LineTraceByChannel Pos (- Pos "0.000000,0.000000,1000.000000") "TraceTypeQuery1" false 0 "None"))
  (bind _height (CallFunction|TimetoHeight (* beat 0.5) 0.4))
  (bind _returnvalue (Game|SpawnActorfromClass "/Game/Assets/Sphere/TutorialSphere.TutorialSphere_C" (Math|Transform|MakeTransform (+ (.location _outhit) (Math|Vector|MakeVector 0.0 0.0 (+ _height (* (.Size (Utilities|Struct|BreakSphereInfoStruct SI)) 7.5)))) "0, 0, 0" "1.000000,1.000000,1.000000") "Undefined" "MultiplyWithRoot" (Components|GetOwner) SI 0))
  (Transformation|AttachActorToActor _returnvalue self "None" "KeepWorld" "KeepWorld" "KeepWorld" true)
  (Utilities|Array|Add (Variables|Default|GetSphereArray) _returnvalue))

(fn DestroyAll
  (for _array_element (Variables|Default|GetSphereArray)
    (Actor|DestroyActor _array_element))
  (Actor|DestroyActor))